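; Collectible note pickup that records its paper name on the player when picked up.
; Box overlap with BP_Player enables input and shows an "E" prompt; leaving clears the prompt but never disables input.
; Interact adds the name to the player's NotesAdded, stores the returned index as Amountofnotes, plays a sound at world origin and destroys the actor.
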(event OnComponentBeginOverlap(Box)
  (params (OverlappedComponent :type Primitive%20Component%20Object%20Reference) (OtherActor :type Actor%20Object%20Reference) (OtherComp :type Primitive%20Component%20Object%20Reference) (OtherBodyIndex :type Integer) (bFromSweep :type Boolean) (SweepResult :type Hit%20Result%20Structure%20%28by%20ref%29))
  (bind _asbp_player (Utilities|Casting|CastToBP_Player OtherActor))
  (Input|EnableInput (Game|GetPlayerController 0))
  (Variables|/Game/Blueprints/BP_Player.BP_Player_C|SetCurrentInteractText _asbp_player "E "))

(event OnComponentEndOverlap(Box)
  (params (OverlappedComponent :type Primitive%20Component%20Object%20Reference) (OtherActor :type Actor%20Object%20Reference) (OtherComp :type Primitive%20Component%20Object%20Reference) (OtherBodyIndex :type Integer))
  (bind _asbp_player (Utilities|Casting|CastToBP_Player OtherActor))
  (Variables|/Game/Blueprints/BP_Player.BP_Player_C|SetCurrentInteractText _asbp_player " "))

(event EventBeginPlay)

(event Collision|EventActorBeginOverlap
  (params (OtherActor :type Actor%20Object%20Reference)))

(event EventTick
  (params (DeltaSeconds :type Float%20%28single-precision%29)))

(event Input|ActionEvents|InputActionInteract
  (params (Key :type Key%20Structure :default "None"))
  (:Pressed
    (bind _asbp_player (Utilities|Casting|CastToBP_Player (stale OnComponentBeginOverlap(Box) OtherActor)))
    (bind _returnvalue (Utilities|Array|Add (Variables|/Game/Blueprints/BP_Player.BP_Player_C|GetNotesAdded _asbp_player) (Variables|Default|Getnameofpaper)))
    (Variables|Default|Setamountofnotes _returnvalue)
    (Audio|PlaySoundatLocation "/Game/PrototypeWeap/Sound/GrenadeLauncher/GL_Bounce03.GL_Bounce03" "0, 0, 0" "0, 0, 0" 1.0 1.0 0.0 0 0 0 0)
    (Actor|DestroyActor)))

(fn ConstructionScript)