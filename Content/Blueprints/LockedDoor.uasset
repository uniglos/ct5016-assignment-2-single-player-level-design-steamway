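; LockedDoor is a sliding door that the player opens with Interact when their NeededKeys array holds this door's NeededKey.
; A trigger box enables input and shows the interact prompt while the player overlaps it.
; A successful key check plays the DoorOpen timeline, which slides the door's relative location.
; When the player leaves the trigger, input is disabled, the prompt clears and the timeline reverses to close the door.
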(event OnComponentBeginOverlap(TriggerBox)
  (params (OverlappedComponent :type Primitive%20Component%20Object%20Reference) (OtherActor :type Actor%20Object%20Reference) (OtherComp :type Primitive%20Component%20Object%20Reference) (OtherBodyIndex :type Integer) (bFromSweep :type Boolean) (SweepResult :type Hit%20Result%20Structure%20%28by%20ref%29))
  ;[1 1 1] on overlap enable input and set text
  (bind _asbp_player (Utilities|Casting|CastToBP_Player OtherActor)
    (:then
      (Input|EnableInput (Game|GetPlayerController 0))
      (Variables|/Game/Blueprints/BP_Player.BP_Player_C|SetCurrentInteractText _asbp_player "E - Open Door"))
    (:CastFailed
      (Utilities|Casting|CastToBP_GuardEnemy OtherActor))))

(event OnComponentEndOverlap(TriggerBox)
  (params (OverlappedComponent :type Primitive%20Component%20Object%20Reference) (OtherActor :type Actor%20Object%20Reference) (OtherComp :type Primitive%20Component%20Object%20Reference) (OtherBodyIndex :type Integer))
  ;[1 1 1] disable input
  (bind _asbp_player (Utilities|Casting|CastToBP_Player OtherActor))
  (Input|DisableInput (Game|GetPlayerController 0))
  (Variables|/Game/Blueprints/BP_Player.BP_Player_C|SetCurrentInteractText _asbp_player "")
  (bind _doorslide (Timeline|DoorOpen Reverse)
    (:Update
      (Transformation|SetRelativeLocation (Variables|Default|GetDoor) _doorslide false false))))

(event Input|ActionEvents|InputActionInteract
  (params (Key :type Key%20Structure :default "None"))
  ;[1 1 1] foreach keys in the needed keys array check if the needed key for this door is in it
  (:Pressed
    (if true
      (bind _asbp_player (Utilities|Casting|CastToBP_Player (Game|GetPlayerCharacter 0)))
      (for (_ _array_index) (Variables|/Game/Blueprints/BP_Player.BP_Player_C|GetNeededKeys _asbp_player)
        (if (Utilities|Enum|Equal(Enum) (Utilities|String|ToString(Integer) _array_index) (Utilities|String|ToString(Integer) (Utilities|Array|FindItem (Variables|/Game/Blueprints/BP_Player.BP_Player_C|GetNeededKeys _asbp_player) (Variables|Default|GetNeeded%20key))))
          (bind _doorslide (Timeline|DoorOpen Play)
            (:Update
              (Transformation|SetRelativeLocation (Variables|Default|GetDoor) _doorslide false false))))))))

(fn ConstructionScript)