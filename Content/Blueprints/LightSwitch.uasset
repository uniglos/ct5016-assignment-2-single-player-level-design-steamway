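; LightSwitch is an interactable that lets the player permanently switch off an assigned array of lights.
; A Box overlap with BP_Player sets the "E" prompt and enables interaction, and ending any overlap disables it without clearing the prompt.
; Tick polls the E key while enabled to zero the lights' intensity and latch LightsOff; until then, it reapplies their on intensity every frame.
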(event OnComponentBeginOverlap(Box)
  (params (OverlappedComponent :type Primitive%20Component%20Object%20Reference) (OtherActor :type Actor%20Object%20Reference) (OtherComp :type Primitive%20Component%20Object%20Reference) (OtherBodyIndex :type Integer) (bFromSweep :type Boolean) (SweepResult :type Hit%20Result%20Structure%20%28by%20ref%29))
  (bind _asbp_player (Utilities|Casting|CastToBP_Player OtherActor))
  (Variables|/Game/Blueprints/BP_Player.BP_Player_C|SetCurrentInteractText _asbp_player "E ")
  (Variables|Default|SetcanpressInteract true))

(event OnComponentEndOverlap(Box)
  (params (OverlappedComponent :type Primitive%20Component%20Object%20Reference) (OtherActor :type Actor%20Object%20Reference) (OtherComp :type Primitive%20Component%20Object%20Reference) (OtherBodyIndex :type Integer))
  (Variables|Default|SetcanpressInteract false))

(event EventTick
  (params (DeltaSeconds :type Float%20%28single-precision%29))
  (Utilities|FlowControl|Sequence
    (:then_0
      (if (Variables|Default|GetcanpressInteract)
        (if (Game|Player|IsInputKeyDown (Game|GetPlayerController 0) "E")
          (for _array_element (Variables|Default|Getlights)
            (Rendering|Components|Light|SetIntensity (Variables|/Script/Engine.PointLight|GetPointLightComponent _array_element) 0.0)
            (Variables|Default|Setlights%20off true)))))
    (:then_1
      (if (not (Variables|Default|Getlights%20off))
        (for _array_element_2 (Variables|Default|Getlights)
          (Rendering|Components|Light|SetIntensity (Variables|/Script/Engine.PointLight|GetPointLightComponent _array_element_2) 1.0))))))

(event Input|ActionEvents|InputActionInteract
  (params (Key :type Key%20Structure :default "None")))

(fn ConstructionScript)